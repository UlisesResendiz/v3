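; BP_Rock1 is a rock actor whose mesh comes from a StaticMesh variable.
; The Construction Script assigns that mesh to the Rock component.
; Tick increments the roll of a stored Rotation variable each frame, independent of delta time, and zeroes pitch and yaw.
; The SetWorldRotation call in the Construction Script is disconnected, so this file never applies that rotation to a component.
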(event `self.ReceiveTick`
  (params (DeltaSeconds :type "Float (single-precision)"))
  (bind _rotation_roll (`KismetMathLibrary.BreakRotator` (`self.rotation`)))
  (bind _result (`/Engine/EditorBlueprintResources/StandardMacros.IncrementFloat` _rotation_roll)
    (:`  `
      (set `self.rotation` (`KismetMathLibrary.MakeRotator` _result)))))

(fn `UserConstructionScript`
  (`StaticMeshComponent.SetStaticMesh` (`self.Rock`) (`self.Static Mesh`)))